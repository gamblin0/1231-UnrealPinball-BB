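; BP_PinballGameState is a pinball game state Blueprint that handles score and ball count changes.
; SetScore stores the new score, while SetBalls assigns NewBalls; each then broadcasts the value through its OnScoreChanged or OnBallsChanged dispatcher and prints it on screen for debugging.
; BeginPlay and the construction script are empty, and leftover test calls to both setters are never executed.
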(event Custom|SetScore
  (params (NewScore :type Float%20%28double-precision%29))
  (bind _output_get (Variables|Default|SetScore NewScore))
  (Default|CallOnScoreChanged _output_get)
  (Development|PrintString (Utilities|String|ToString(Float) _output_get) true true "(R=1.000000,G=0.000000,B=0.849804,A=1.000000)"))

(event Custom|SetBalls
  (params (NewBalls :type Integer))
  (bind _output_get (Variables|Default|SetNew%20Balls NewBalls))
  (Default|CallOnBallsChanged _output_get)
  (Development|PrintString (Utilities|String|ToString(Integer) _output_get)))

(event EventBeginPlay)

(fn ConstructionScript)