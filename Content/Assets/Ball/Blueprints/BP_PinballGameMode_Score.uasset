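; Pinball game mode Blueprint that handles adding points to the score.
; Its AddScore event casts the current game state to BP_PinballGameState and sets that state's Score to the existing value plus the incoming points.
; BeginPlay and Tick are disabled placeholders, and the construction script only calls its parent.
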(event EventBeginPlay
  (|CallParentFunction) ; This node is disabled and will not be called.\nDrag off pins to build functionality.
)

(event EventTick
  (params (DeltaSeconds :type Float%20%28single-precision%29))
  (|CallParentFunction DeltaSeconds) ; This node is disabled and will not be called.\nDrag off pins to build functionality.
)

(event EventAddScore
  (params (Points :type Float%20%28double-precision%29))
  (bind _asbp_pinball_game_state (Utilities|Casting|CastToBP_PinballGameState (Game|GetGameState)))
  (Default|SetScore _asbp_pinball_game_state (+ Points (Variables|/Game/Assets/Ball/Blueprints/BP_PinballGameState.BP_PinballGameState_C|GetScore _asbp_pinball_game_state))))

(fn ConstructionScript
  (|CallParentFunction))