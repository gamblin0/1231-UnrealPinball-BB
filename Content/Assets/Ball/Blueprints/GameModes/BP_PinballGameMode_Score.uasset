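; Pinball game mode that handles scoring and lost balls, keeping both values in BP_PinballGameState.
; AddScore adds the given points to the current score through the game state's SetScore.
; OnBallLost decrements the remaining balls, updates the count through SetBalls, then calls SpawnBall while any remain.
; When none are left, game over is only a red printed debug message.
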(event EventBeginPlay
  (|CallParentFunction) ; This node is disabled and will not be called.\nDrag off pins to build functionality.
)

(event EventTick
  (params (DeltaSeconds :type Float%20%28single-precision%29))
  (|CallParentFunction DeltaSeconds) ; This node is disabled and will not be called.\nDrag off pins to build functionality.
)

(event EventAddScore
  (params (Points :type Float%20%28double-precision%29))
  (bind _asbp_pinball_game_state (Utilities|Casting|CastToBP_PinballGameState (Game|GetGameState)))
  (Default|SetScore _asbp_pinball_game_state (+ Points (Variables|/Game/Assets/Ball/Blueprints/GameModes/BP_PinballGameState.BP_PinballGameState_C|GetScore _asbp_pinball_game_state))))

(event EventOnBallLost
  (bind _asbp_pinball_game_state (Utilities|Casting|CastToBP_PinballGameState (Game|GetGameState)))
  (bind _result (Math|Integer|DecrementInt (Variables|/Game/Assets/Ball/Blueprints/GameModes/BP_PinballGameState.BP_PinballGameState_C|GetBallsRemaining _asbp_pinball_game_state))
    (:%20%20
      (Default|SetBalls _asbp_pinball_game_state _result)
      (if (> _result 0)
        (CallFunction|SpawnBall)
        (else
          (Development|PrintString "GAME OVER" true true "(R=1.000000,G=0.000000,B=0.000000,A=1.000000)"))))))

(fn ConstructionScript
  (|CallParentFunction))