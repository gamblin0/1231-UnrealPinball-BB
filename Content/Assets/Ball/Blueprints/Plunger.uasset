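; Pinball plunger actor that animates its mesh when activated and released.
; Activation plays a timeline that lerps the plunger mesh's relative location between two points.
; Deactivation stops the timeline and eases the mesh with a short MoveComponentTo.
; The pinball impulse message using MaxForce is disconnected and the overlap event is empty, so the Blueprint applies no launch force.
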(event Custom|OnActivate_Event
  (bind _newtrack_0 (Timeline|Timeline PlayFromStart)
    (:Update
      (Transformation|SetRelativeLocation (Variables|Default|GetSM_Plunger) (Math|Vector|Lerp(Vector) (Variables|Default|GetA) (Variables|Default|GetB) _newtrack_0) false false))))

(event Custom|OnDeactivate_Event
  (Utilities|FlowControl|Sequence
    (:then_0
      (bind _newtrack_0 (Timeline|Timeline Stop)
        (:Update
          (Transformation|SetRelativeLocation (Variables|Default|GetSM_Plunger) (Math|Vector|Lerp(Vector) (Variables|Default|GetA) (Variables|Default|GetB) _newtrack_0) false false))))
    (:then_1
      (Components|MoveComponentTo (Variables|Default|GetSM_Plunger) "0, 0, 0" "0, 0, 0" false false 0.1 false))))

(event EventBeginPlay
  (Variables|Default|SetMaxForce 0.0))

(event Collision|EventActorBeginOverlap
  (params (OtherActor :type Actor%20Object%20Reference)))

(event EventTick
  (params (DeltaSeconds :type Float%20%28single-precision%29)))

(fn ConstructionScript)