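; Pinball plunger actor that charges on activation and launches objects that react to pinball impulses.
; Activation runs a timeline that slides the plunger mesh toward its end position while recording charge; deactivation stops it and animates the mesh back from the reached position.
; When an overlap with the Box ends, BPI_PinballReactive actors receive an impulse directed away from the plunger, scaled by charge and maximum force.
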(event OnComponentEndOverlap(Box)
  (params (OverlappedComponent :type Primitive%20Component%20Object%20Reference) (OtherActor :type Actor%20Object%20Reference) (OtherComp :type Primitive%20Component%20Object%20Reference) (OtherBodyIndex :type Integer))
  (bind _asbpi_pinball_reactive (Utilities|Casting|CastToBPI_PinballReactive OtherActor))
  (Default|PinballImpulseEvent _asbpi_pinball_reactive (* (* (Variables|Default|GetMaxForce) (Variables|Default|GetCharge%20Alpha)) (Math|Vector|Normalize (- (Transformation|GetWorldLocation OtherComp) (Transformation|GetActorLocation))))))

(event Custom|OnActivate_Event
  (bind _charge_alpha (Timeline|Timeline PlayFromStart)
    (:Update
      (Variables|Default|SetCharge%20Alpha _charge_alpha)
      (Variables|Default|SetUpdatedPos (Math|Vector|Lerp(Vector) (Variables|Default|GetStartPos) (Variables|Default|GetEndPos) _charge_alpha))
      (Transformation|SetRelativeLocation (Variables|Default|GetSM_Plunger) (Math|Vector|Lerp(Vector) (Variables|Default|GetStartPos) (Variables|Default|GetEndPos) _charge_alpha) false false))))

(event Custom|OnDeactivate_Event
  (Utilities|FlowControl|Sequence
    (:then_0
      (bind _charge_alpha (Timeline|Timeline Stop)
        (:Update
          (Variables|Default|SetCharge%20Alpha _charge_alpha)
          (Variables|Default|SetUpdatedPos (Math|Vector|Lerp(Vector) (Variables|Default|GetStartPos) (Variables|Default|GetEndPos) _charge_alpha))
          (Transformation|SetRelativeLocation (Variables|Default|GetSM_Plunger) (Math|Vector|Lerp(Vector) (Variables|Default|GetStartPos) (Variables|Default|GetEndPos) _charge_alpha) false false))))
    (:then_1
      (bind _newtrack_0 (Timeline|Timeline_0 PlayFromStart)
        (:Update
          (Transformation|SetRelativeLocation (Variables|Default|GetSM_Plunger) (Math|Vector|Lerp(Vector) (Variables|Default|GetUpdatedPos) (Variables|Default|GetStartPos) _newtrack_0) false false))))))

(fn ConstructionScript)