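; BP_TestBall is a test physics ball Blueprint with a Sphere component that reacts to pinball-style pushes.
; PinballImpulseEvent applies the incoming Force scaled by the sphere's mass through AddForce, without acceleration change.
; Tick reads the sphere's linear velocity but does nothing with it.
; A ball trail Niagara spawn on BeamOffset and a velocity normalization are left unconnected.
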(event EventTick
  (params (DeltaSeconds :type Float%20%28single-precision%29))
  (bind _returnvalue (Physics|GetPhysicsLinearVelocity (Variables|Default|GetSphere) "None")))

(event EventPinballImpulseEvent
  (params (Force :type Vector :default "0, 0, 0"))
  (bind _sphere (Variables|Default|GetSphere))
  (Physics|AddForce _sphere (* Force (Physics|GetMass _sphere)) "None" false))

(fn ConstructionScript)