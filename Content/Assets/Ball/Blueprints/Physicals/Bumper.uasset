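; Pinball pop bumper that knocks reactive actors away and awards score when they touch its capsule.
; On overlap it sends an impulse pointing outward from the bumper through BPI_PinballReactive, then adds score on the game mode via BPI_ScoreReciever.
; A timeline lerps the mechanism mesh between start and end positions for any overlapping actor.
; End overlap stops the timeline and snaps the mesh back to start.
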(event OnComponentBeginOverlap(Capsule)
  (params (OverlappedComponent :type Primitive%20Component%20Object%20Reference) (OtherActor :type Actor%20Object%20Reference) (OtherComp :type Primitive%20Component%20Object%20Reference) (OtherBodyIndex :type Integer) (bFromSweep :type Boolean) (SweepResult :type Hit%20Result%20Structure%20%28by%20ref%29))
  (Utilities|FlowControl|Sequence
    (:then_0
      ;[0.03232 0.1379 0.15 0.5] Bump Impulse
      (bind _asbpi_pinball_reactive (Utilities|Casting|CastToBPI_PinballReactive OtherActor))
      (Default|PinballImpulseEvent _asbpi_pinball_reactive (* (Variables|Default|GetMaxForce) (Math|Vector|Normalize (- (Transformation|GetWorldLocation OtherComp) (Transformation|GetActorLocation)))))
      (bind _asbpi_score_reciever (Utilities|Casting|CastToBPI_ScoreReciever (Game|GetGameMode)))
      (Default|AddScore _asbpi_score_reciever (Variables|Default|GetScoreValue)))
    (:then_1
      ;[0.15 0.1157 0.03394 0.5] Animation
      (bind _newtrack_0 (Timeline|Anim%20Timeline Play)
        (:Update
          (Transformation|SetRelativeLocation (Variables|Default|GetSM_PopBumperMechanism) (Math|Vector|Lerp(Vector) (Variables|Default|GetStartPos) (Variables|Default|GetEndPos) _newtrack_0) false false))))))

(event OnComponentEndOverlap(Capsule)
  (params (OverlappedComponent :type Primitive%20Component%20Object%20Reference) (OtherActor :type Actor%20Object%20Reference) (OtherComp :type Primitive%20Component%20Object%20Reference) (OtherBodyIndex :type Integer))
  ;[0.15 0.1157 0.03394 0.5] Animation
  (Utilities|FlowControl|Sequence
    (:then_0
      (bind _newtrack_0 (Timeline|Anim%20Timeline Stop)
        (:Update
          (Transformation|SetRelativeLocation (Variables|Default|GetSM_PopBumperMechanism) (Math|Vector|Lerp(Vector) (Variables|Default|GetStartPos) (Variables|Default|GetEndPos) _newtrack_0) false false))))
    (:then_1
      (Transformation|SetRelativeLocation (Variables|Default|GetSM_PopBumperMechanism) (Variables|Default|GetStartPos) false false))))

(fn ConstructionScript)