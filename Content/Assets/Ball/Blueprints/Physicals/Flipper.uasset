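; Flipper is a physical ball-game Blueprint that swings its Flipper component between a rest rotation and a rotated end position.
; BeginPlay sets the rest to zero rotation and uses the Direction enum to pick a quarter-turn end rotation in either direction.
; OnActivate plays a timeline that lerps the component's relative rotation toward the end, and OnDeactivate reverses it to swing back.
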(event Custom|OnActivate
  (bind _newtrack_0 (Timeline|Timeline Play)
    (:Update
      (Transformation|SetRelativeRotation (Variables|Default|GetFlipper) (Math|Rotator|Lerp(Rotator) (Variables|Default|GetStartRot) (Variables|Default|GetEndRot) _newtrack_0) false false))))

(event Custom|OnDeactivate
  (bind _newtrack_0 (Timeline|Timeline Reverse)
    (:Update
      (Transformation|SetRelativeRotation (Variables|Default|GetFlipper) (Math|Rotator|Lerp(Rotator) (Variables|Default|GetStartRot) (Variables|Default|GetEndRot) _newtrack_0) false false))))

(event EventBeginPlay
  (bind _output_get (Variables|Default|SetStartRot "0, 0, 0"))
  (Variables|Default|SetEndRot (Math|Rotator|CombineRotators _output_get (Math|Rotator|SelectRotator "0.000000,-90.000000,0.000000" "0.000000,90.000000,0.000000" (Utilities|Enum|Equal(Enum) (Variables|Default|GetDirection) "NewEnumerator0")))))

(fn ConstructionScript)